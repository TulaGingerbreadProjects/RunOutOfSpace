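; Letter actor that displays one text character and acts as a jump or launch trigger for ROS_Char.
; The construction script writes Letter to the TextRender and flags it as a space (an empty literal) or a dot.
; When ROS_Char overlaps the Trigger, a space makes it jump and a dot launches it straight up.
; Other letters have no overlap effect.
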(event OnComponentBeginOverlap(Trigger)
  (params (OverlappedComponent :type Primitive%20Component%20Object%20Reference) (OtherActor :type Actor%20Object%20Reference) (OtherComp :type Primitive%20Component%20Object%20Reference) (OtherBodyIndex :type Integer) (bFromSweep :type Boolean) (SweepResult :type Hit%20Result%20Structure%20%28by%20ref%29))
  (bind _asros_char (Utilities|Casting|CastToROS_Char OtherActor))
  (if (Variables|Default|GetisSpace)
    (Character|Jump _asros_char)
    (elif (Variables|Default|GetisDot)
      (Character|LaunchCharacter _asros_char "0, 0,2000.000000" false false))))

(fn ConstructionScript
  (Variables|Default|SetisSpace (Utilities|Enum|Equal(Enum) (Variables|Default|GetLetter) (Utilities|Text|MakeLiteralText " ")))
  (Variables|Default|SetisDot (Utilities|Enum|Equal(Enum) (Variables|Default|GetLetter) (Utilities|Text|MakeLiteralText ".")))
  (Rendering|Components|TextRender|SetText (Variables|Default|GetTextRender) (Variables|Default|GetLetter)))