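; Typing-game component that turns key presses into Letter actors laid out in a line, matched against the current word's accepted variants.
; Words advance through looping texts and sentences, refreshing HUD hints and maximum length while completed letters remain in the world.
; Backspace removes the last letter; exceeding the longest variant deletes the attempt and launches the owning Character backwards, scaled by its length.
; Letter spacing is measured at startup from a temporary Letter.
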(event EventBeginPlay
  (Manager|Initialize))

(fn IsLetter
  (params (InputPin :type Key%20Structure%20%28by%20ref%29))
  (LocalVariables|Setlocal_isLetter false)
  (if (Class|KismetInputLibrary|KeyIsKeyboardKey InputPin)
    (for _array_element (LocalVariables|GetAlphabet)
      (if (Utilities|Enum|Equal(Enum) _array_element (Class|KismetInputLibrary|KeyGetDisplayName InputPin))
        (LocalVariables|Setlocal_isLetter true)))
    (return (LocalVariables|Getlocal_isLetter) InputPin)))

(fn HandleKeyPressed
  (params (Key :type Key%20Structure))
  (bind (_isletter _letter) (Letter|IsLetter Key))
  (if _isletter
    (Letter|SpawnLetter (Class|KismetInputLibrary|KeyGetDisplayName _letter))
    (Word|AddLettertoWord (Class|KismetInputLibrary|KeyGetDisplayName _letter))
    (Word|CheckWord)
    (Development|PrintText (Variables|Word|GetcurWord) true true "(R=0.500000,G=0.000000,B=0.500000,A=1.000000)") ; DEBUG: PRINT CURRENT WORD
    (elif (== _letter "BackSpace")
      (Letter|DeleteLetter)
      (else
        ;[0.5 0 0.5] DEBUG: SPACE FOR TESTS
        (if (== _letter "SpaceBar")
          (Letter|SpawnLetter " ")
          (Development|PrintText "SPACE BAR" true true "(R=0.500000,G=0.000000,B=0.500000,A=1.000000)") ; DEBUG: PRINT WHEN SPACE PRESSED
          (Variables|Word|SetcurWord ""))))))

(fn SpawnLetter
  (params (Letter :type Text))
  (bind _output_get (Variables|Letter|SetnextLetterLocation (+ (Variables|Letter|GetnextLetterLocation) (Variables|Letter|GetletterSize))))
  (bind _returnvalue (Game|SpawnActorfromClass "/Game/Blueprints/Letters/Letter.Letter_C" (Math|Transform|MakeTransform _output_get "0, 0, 0" "1,1,1") "Undefined" 0 Letter 0))
  (Utilities|Array|Add (Variables|Letter|GetLetterRefs) _returnvalue))

(fn DeleteLetter
  (bind _letterrefs (Variables|Letter|GetLetterRefs))
  (bind _returnvalue (Utilities|Array|LastIndex _letterrefs))
  (bind _output (Utilities|Array|Get(acopy) _letterrefs _returnvalue))
  (Utilities|IsValid _output
    (:Is%20Valid
      (Actor|DestroyActor _output)
      (Utilities|Array|RemoveIndex (Variables|Letter|GetLetterRefs) _returnvalue)
      (Variables|Letter|SetnextLetterLocation (- (Variables|Letter|GetnextLetterLocation) (Variables|Letter|GetletterSize)))
      (Word|RemoveLastLetter))))

(fn CheckWord
  (if (<= (Utilities|String|Len (Utilities|String|ToString(Text) (Variables|Word|GetcurWord))) (Variables|Word|GetmaxLen))
    (for _array_element (Utilities|Struct|Breakword_S (Text|GetCurrentWord))
      (if (Utilities|Enum|Equal(Enum) _array_element (Variables|Word|GetcurWord))
        (|CorrectWord)))
    (else
      (|WrongWord))))

(fn Initialize
  (Utilities|FlowControl|Sequence
    (:then_0
      (Default|UpdateWordHints (Variables|/Game/Blueprints/UMG/HUD_W.HUD_W_C|GetWordHintsBox (Variables|Manager|GetHUD_ref)) (Utilities|Struct|Breakword_S (Text|GetCurrentWord))))
    (:then_1
      (Word|UpdateMaxLength))
    (:then_2
      ;[0 0.5 0] Set LetterSize in dynamic
      (bind _returnvalue (Game|SpawnActorfromClass "/Game/Blueprints/Letters/Letter.Letter_C" (Math|Transform|MakeTransform "0, 0, 0" "0, 0, 0" "1,1,1") "Undefined" 0 "L" 0))
      (Variables|Letter|SetletterSize (Math|Vector|MakeVector (+ (.x (/ (Class|TextRenderComponent|GetTextWorldSize (Variables|/Game/Blueprints/Letters/Letter.Letter_C|GetLetterTextRender _returnvalue)) 2)) (.y (/ (Class|TextRenderComponent|GetTextWorldSize (Variables|/Game/Blueprints/Letters/Letter.Letter_C|GetLetterTextRender _returnvalue)) 2)) (.z (/ (Class|TextRenderComponent|GetTextWorldSize (Variables|/Game/Blueprints/Letters/Letter.Letter_C|GetLetterTextRender _returnvalue)) 2))) 0.0 0.0))
      (Actor|DestroyActor _returnvalue))))

(fn GetCurrentWord
  (return (Utilities|Array|Get(acopy) (.words (Utilities|Array|Get(acopy) (.sentences (Utilities|Array|Get(acopy) (Variables|Text|GetTexts) (Variables|Text|GettextIndex))) (Variables|Text|GetsentenceIndex))) (Variables|Text|GetwordIndex))))

(fn GetCurrentSentence
  (return (Utilities|Array|Get(acopy) (.sentences (Utilities|Array|Get(acopy) (Variables|Text|GetTexts) (Variables|Text|GettextIndex))) (Variables|Text|GetsentenceIndex))))

(fn GetCurrentText
  (return (Utilities|Array|Get(acopy) (Variables|Text|GetTexts) (Variables|Text|GettextIndex))))

(fn AddLettertoWord
  (params (newLetter :type Text%20%28by%20ref%29))
  (Variables|Word|SetcurWord (Utilities|Text|FormatText "{Word}{Letter}" (Variables|Word|GetcurWord) newLetter)))

(fn UpdateMaxLength
  (LocalVariables|Setlocal_max 0)
  (for _array_element (Utilities|Struct|Breakword_S (Text|GetCurrentWord))
    (if (< (LocalVariables|Getlocal_max) (Utilities|String|Len (Utilities|String|ToString(Text) _array_element)))
      (LocalVariables|Setlocal_max (Utilities|String|Len (Utilities|String|ToString(Text) _array_element)))))
  (Variables|Word|SetmaxLen (LocalVariables|Getlocal_max))
  (return))

(fn RemoveLastLetter
  (Variables|Word|SetcurWord (Utilities|Text|ToText(String) (Utilities|String|GetSubstring (Utilities|String|ToString(Text) (Variables|Word|GetcurWord)) 0 (- (Utilities|String|Len (Utilities|String|ToString(Text) (Variables|Word|GetcurWord))) 1)))))