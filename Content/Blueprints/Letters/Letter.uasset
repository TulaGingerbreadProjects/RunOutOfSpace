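; Letter actor that displays a character in the world and acts as a jump pad when it represents the space bar.
; The construction script writes Letter to a text render component and sets IsSpace when Letter equals an empty text literal.
; When a ROS_Character overlaps JumpTrigger on a space letter, the actor calls Jump on that character.
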(event OnComponentBeginOverlap(JumpTrigger)
  (params (OverlappedComponent :type Primitive%20Component%20Object%20Reference) (OtherActor :type Actor%20Object%20Reference) (OtherComp :type Primitive%20Component%20Object%20Reference) (OtherBodyIndex :type Integer) (bFromSweep :type Boolean) (SweepResult :type Hit%20Result%20Structure%20%28by%20ref%29))
  (bind _asros_character (Utilities|Casting|CastToROS_Character OtherActor))
  (if (Variables|Default|GetisSpace)
    (Character|Jump _asros_character)))

(fn ConstructionScript
  (Variables|Default|SetisSpace (Utilities|Enum|Equal(Enum) (Variables|Default|GetLetter) (Utilities|Text|MakeLiteralText " ")))
  (Rendering|Components|TextRender|SetText (Variables|Default|GetLetterTextRender) (Variables|Default|GetLetter)))