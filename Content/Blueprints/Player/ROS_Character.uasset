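; Player character for what appears to be a 2D auto-runner typing game, moving constantly along world +X.
; A looping timer set on BeginPlay is meant to raise max walk speed every second, with no cap.
; Tick applies the movement input and switches the sprite between running and idle flipbooks based on velocity.
; Typed key presses are forwarded to WordsManager for handling.
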(event Custom|increaseSpeed
  (bind _charactermovement (Variables|Character|GetCharacterMovement))
  ;[1 1 1] Add max speed
  (Variables|/Script/Engine.CharacterMovementComponent|SetMaxWalkSpeed _charactermovement (+ (Variables|/Script/Engine.CharacterMovementComponent|GetMaxWalkSpeed _charactermovement) 1e+02)))

(event EventBeginPlay
  ;[1 1 1] Set timer to increase speed
  (Utilities|Time|SetTimerbyEvent (EventDispatchers|CreateEvent :!event Custom|increaseSpeed) 1.0 true))

(event EventTick
  (params (DeltaSeconds :type Float%20%28single-precision%29))
  ;[1 1 1] Tick - Updates animation
  (Pawn|Input|AddMovementInput "1.000000, 0, 0" 1.0 false)
  (CallFunction|UpdateAnimation))

(event Input|ActionEvents|InputActionTypeText
  (params (Key :type Key%20Structure))
  ;[1 1 1] OnTextTyping
  (:Pressed
    (Default|HandleKeyPressed (Variables|Default|GetWordsManager) Key)))

(fn ConstructionScript)

(fn UpdateAnimation
  (Sprite|SetFlipbook (Variables|Default|GetSprite) (select (> (Math|Vector|VectorLength (Transformation|GetVelocity)) 0.0) "/Game/Assets/Sprites/RunningAnimation.RunningAnimation" "/Game/Assets/Sprites/IdleAnimation.IdleAnimation")))